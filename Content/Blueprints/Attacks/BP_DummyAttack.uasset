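; BP_DummyAttack is a cursor-following stand-in for the player's selected attack, sized to that attack's radius.
; On BeginPlay it reads CurrentAttack from the ProtagClass player and scales its static mesh from the matching Lightning Bolt, Fireball or Dark Whirl radius.
; Every tick it teleports AtkHitBox to the complex Visibility-trace hit under the mouse cursor.
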(event EventBeginPlay
  (bind _staticmesh (Variables|Default|GetStaticMesh))
  ;[1 1 1] Set size of collider
  (Variables|Default|SetRadiusToScale (/ 0.625 32.0))
  (bind _asprotag_class (Utilities|Casting|CastToProtagClass (Game|GetPlayerCharacter 0)))
  (switch string (Variables|/Script/HSPGame.ProtagClass|GetcurrentAttack _asprotag_class)
    (:LightningBolt
      (Transformation|SetWorldScale3D _staticmesh (Math|Conversions|ToVector(Float) (* (Variables|Default|GetradiusLightningBolt) (Variables|Default|GetRadiusToScale)))))
    (:Fireball
      (Transformation|SetWorldScale3D _staticmesh (Math|Conversions|ToVector(Float) (* (Variables|Default|GetradiusFireBall) (Variables|Default|GetRadiusToScale)))))
    (:DarkWhirl
      (Transformation|SetWorldScale3D _staticmesh (Math|Conversions|ToVector(Float) (* (Variables|Default|GetRadiusToScale) (Variables|Default|GetradiusDarkWhirl)))))))

(event EventTick
  (params (DeltaSeconds :type Float%20%28single-precision%29))
  ;[1 1 1] Update position of collider
  (Transformation|SetWorldLocation (Variables|Default|GetatkHitBox) (.Location (Collision|BreakHitResult (.HitResult (Game|Player|GetHitResultUnderCursorbyChannel (Game|GetPlayerController 0) "TraceTypeQuery1" true)))) false true))

(fn ConstructionScript)