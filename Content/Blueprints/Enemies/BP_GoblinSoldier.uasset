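; BP_GoblinSoldier is a goblin soldier enemy pawn for what appears to be turn-based combat.
; Every Tick it stops movement once CurrHealth drops to zero or below.
; While IsBattling, it uses AIMoveTo toward the player on its turn and halts immediately when IsTurn is false.
; The construction script is empty.
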(event EventTick
  (params (DeltaSeconds :type Float%20%28single-precision%29))
  (if (<= (Variables|Default|GetcurrHealth) 0.0) ; If Dead
    (Components|Movement|StopMovementImmediately (Variables|Character|GetCharacterMovement))
    (elif (Variables|Default|GetisBattling)
      (if (Variables|Default|GetisTurn)
        (AI|AIMoveTo self "0, 0, 0" (Game|GetPlayerCharacter 0) 5.0 false)
        (else
          (Components|Movement|StopMovementImmediately (Variables|Character|GetCharacterMovement)))))))

(fn ConstructionScript)