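; Player character Blueprint that creates the HUD, opens and closes the Arms Dealer shop, and fades meshes blocking the camera indoors.
; The talk input opens the shop for any dealer with CanTalk set.
; A looping timer box-traces from camera to player, with box orientation chosen by IsInside and IsInsideHorizontal.
; Hit static mesh actors are compared with the previously hidden set to toggle their BP_FadeComponents.
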(event Custom|Close%20Shop
  ;[1 1 1] Close Shop UI Custom Event
  (Widget|RemovefromParent (stale Input|ActionEvents|InputActionTalkAction _returnvalue)))

(event EventBeginPlay
  (bind _returnvalue (UserInterface|CreateWidget "/Game/UI/playerHud.playerHud_C"))
  (UserInterface|Viewport|AddtoViewport _returnvalue 0)
  (Utilities|Time|SetTimerbyFunctionName 0 "UpdateFadeActors" 0.2 true) ; Call the listed function every interval set in time
)

(event Collision|EventActorBeginOverlap
  (params (OtherActor :type Actor%20Object%20Reference)))

(event Input|ActionEvents|InputActionTalkAction
  (params (Key :type Key%20Structure))
  ;[1 1 1] Open up the shop UI
  (:Pressed
    (bind _outactors (Actor|GetAllActorsOfClass "/Game/Blueprints/Characters/BP_ArmsDealerClass.BP_ArmsDealerClass_C")) ; Check all Arms Dealers
    (for _array_element _outactors
      (if (Variables|/Script/HSPGame.ArmsDealerClass|GetcanTalk _array_element) ; If one can talk open up the shop\nUI
        (bind _returnvalue (UserInterface|CreateWidget "/Game/UI/ShopScreen.shopScreen_C"))
        (UserInterface|Viewport|AddtoViewport _returnvalue 0)))))

(event Input|MouseEvents|LeftMouseButton
  (params (Key :type Key%20Structure)))

(fn ConstructionScript)

(fn UpdateFadeActors
  (Utilities|FlowControl|Sequence
    (:then_0
      (if (Variables|Default|GetisInside)
        (Utilities|FlowControl|Sequence
          (:then_0
            (Utilities|Array|Clear (Variables|Default|GetHitMeshes)) ; Clear the hit meshes first
          )
          (:then_1
            (bind (_outhits _returnvalue) (Class|KismetSystemLibrary|BoxTraceMultiforObjects (Transformation|GetWorldLocation (Variables|Default|GetCamera)) (Transformation|GetActorLocation) "20.000000,500.000000, 0" "0, 0, 0" (Utilities|Array|MakeArray "ObjectTypeQuery1") false 0 "None" true)) ; Trace from camera to player and store all hit static meshes
            (if _returnvalue
              (for _array_element _outhits
                (bind _asstatic_mesh_actor (Utilities|Casting|CastToStaticMeshActor (.HitActor (Collision|BreakHitResult _array_element))))
                (Utilities|Array|AddUnique (Variables|Default|GetHitMeshes) _asstatic_mesh_actor)
                (CallFunction|SetShownMeshes)
                (CallFunction|SetHiddenMeshes))
              (else
                (CallFunction|SetShownMeshes)))))
        (else
          (Utilities|Array|Clear (Variables|Default|GetHitMeshes)) ; Clear the hit meshes first
        )))
    (:then_1
      (if (Variables|Default|GetisInsideHorizontal)
        (Utilities|FlowControl|Sequence
          (:then_0
            (Utilities|Array|Clear (Variables|Default|GetHitMeshes)) ; Clear the hit meshes first
          )
          (:then_1
            (bind (_outhits_2 _returnvalue_2) (Class|KismetSystemLibrary|BoxTraceMultiforObjects (Transformation|GetWorldLocation (Variables|Default|GetCamera)) (Transformation|GetActorLocation) "500.000000,20.000000, 0" "0, 0, 0" (Utilities|Array|MakeArray "ObjectTypeQuery1") false 0 "None" true)) ; Trace from camera to player and store all hit static meshes
            (if _returnvalue_2
              (for _array_element_2 _outhits_2
                (bind _asstatic_mesh_actor_2 (Utilities|Casting|CastToStaticMeshActor (.HitActor (Collision|BreakHitResult _array_element_2))))
                (Utilities|Array|AddUnique (Variables|Default|GetHitMeshes) _asstatic_mesh_actor_2)
                (CallFunction|SetShownMeshes)
                (CallFunction|SetHiddenMeshes))
              (else
                (CallFunction|SetShownMeshes)))))
        (else
          (Utilities|Array|Clear (Variables|Default|GetHitMeshes)) ; Clear the hit meshes first
        )))))

(fn SetShownMeshes
  (for _array_element (Variables|Default|GetHiddenMeshes)
    (if (not (Utilities|Array|ContainsItem (Variables|Default|GetHitMeshes) _array_element))
      (for _array_element_2 (Actor|GetComponentsByClass _array_element "/Game/Blueprints/FadeStaticMesh/BP_FadeComponent.BP_FadeComponent_C")
        (Default|ToggleHideMesh _array_element_2 false)))))

(fn SetHiddenMeshes
  (bind _output_get (Variables|Default|SetHiddenMeshes (Variables|Default|GetHitMeshes)))
  (for _array_element _output_get
    (for _array_element_2 (Actor|GetComponentsByClass _array_element "/Game/Blueprints/FadeStaticMesh/BP_FadeComponent.BP_FadeComponent_C")
      (Default|ToggleHideMesh _array_element_2 true))))