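; Slime enemy character that moves toward the player while its IsTurn flag is set.
; BeginPlay stops it rotating by turning off controller yaw and zeroing the movement rotation rate, though orient-to-movement is on.
; Tick reissues AI MoveTo on the first player character every frame during its turn; nothing in this Blueprint sets that flag.
; Both events also print a debug greeting.
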(event EventBeginPlay
  (bind _charactermovement (Variables|Character|GetCharacterMovement))
  (Development|PrintString "Hello")
  (Variables|Default|SetbUseControllerRotationYaw false) ; Prevent Enemy from rotating
  (Variables|/Script/Engine.CharacterMovementComponent|SetbOrientRotationToMovement _charactermovement true)
  (Variables|/Script/Engine.CharacterMovementComponent|SetRotationRate _charactermovement "0, 0, 0") ; Speed of rotation
)

(event Collision|EventActorBeginOverlap
  (params (OtherActor :type Actor%20Object%20Reference)))

(event EventTick
  (params (DeltaSeconds :type Float%20%28single-precision%29))
  (if (Variables|Default|GetisTurn)
    (Development|PrintString "Hello")
    (AI|AIMoveTo self "0, 0, 0" (Game|GetPlayerCharacter 0) 5.0 false)))

(fn ConstructionScript)