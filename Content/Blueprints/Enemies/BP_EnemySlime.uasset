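; BP_EnemySlime is an enemy slime character that takes part in battles and carries its own HUD widget.
; On BeginPlay it casts the widget component's object to slimeHud and passes it a reference to itself.
; Each tick while battling, it uses AI MoveTo toward the player on its turn and halts its movement immediately otherwise.
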(event EventBeginPlay
  (bind _asslime_hud (Utilities|Casting|CastToslimeHud (UserInterface|GetUserWidgetObject (Variables|Default|GetslimeHUDComp))))
  (Variables|/Game/UI/slimeHud.slimeHud_C|SetenemySlimeBP _asslime_hud self))

(event Collision|EventActorBeginOverlap
  (params (OtherActor :type Actor%20Object%20Reference)))

(event EventTick
  (params (DeltaSeconds :type Float%20%28single-precision%29))
  (if (Variables|Default|GetisBattling)
    (if (Variables|Default|GetisTurn)
      (AI|AIMoveTo self "0, 0, 0" (Game|GetPlayerCharacter 0) 5.0 false)
      (else
        (Components|Movement|StopMovementImmediately (Variables|Character|GetCharacterMovement)) ; Stop the characters movement
      ))))

(fn ConstructionScript)