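; Base-style 2D flipbook enemy with a floating hover-info widget, which receives a self reference on BeginPlay for its bindings.
; Each Tick flips the sprite by Y velocity and picks an idle, walk or death flipbook through a small state function driven by movement and health.
; While alive and battling, it moves toward the player on its turn and otherwise stops.
; At zero health it stops and hides the widget.
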(event Custom|UpdateAnimation
  (bind _sprite (Variables|Default|GetSprite))
  ;[1 1 1] Custom Update Animation Function, Sets Flipbook
  (if (< (.Y (Math|Vector|BreakVector (Transformation|GetVelocity))) 0.0) ; Set the rotation of the sprite so\nit faces left or right
    (Transformation|SetRelativeRotation _sprite "0,90.000000, 0" false false) ; Flip the sprite to face right when moving\nin a positive horizontal direction
    (else
      (Transformation|SetRelativeRotation _sprite "0,-90.000000, 0" false false) ; Reset to default direction (Left)
    ))
  (bind _output_get (Variables|Default|SetisMoving (> (Math|Vector|VectorLength (Transformation|GetVelocity)) 0.0))) ; Check if the enemy is\nmoving and update this bool
  (bind _output_fb (CallFunction|AnimStateMachine _output_get (<= (Variables|Default|GetcurrHealth) 0.0))) ; Call the State machine function and get\na FlipBook
  (Sprite|SetFlipbook (Variables|Default|GetSprite) _output_fb) ; Update the current Flipbook for the BP
)

(event EventBeginPlay
  ;[1 1 1] Pass a reference to self to the UI so bindings work
  (bind _asenemy_hover_info (Utilities|Casting|CastToenemyHoverInfo (UserInterface|GetUserWidgetObject (Variables|Default|GetenemyInfoWidget))))
  (Variables|/Game/UI/enemyHoverInfo.enemyHoverInfo_C|SetenemyBP _asenemy_hover_info self))

(event Collision|EventActorBeginOverlap
  (params (OtherActor :type Actor%20Object%20Reference)))

(event EventTick
  (params (DeltaSeconds :type Float%20%28single-precision%29))
  ;[1 1 1] Tick
  (CallFunction|UpdateAnimation) ; Set the current BP's flipbook
  (if (<= (Variables|Default|GetcurrHealth) 0.0)
    (Components|Movement|StopMovementImmediately (Variables|Character|GetCharacterMovement))
    (Rendering|SetVisibility (Variables|Default|GetenemyInfoWidget) false false) ; Hide the enemy floating UI on death
    (elif (Variables|Default|GetisBattling)
      (if (Variables|Default|GetisTurn)
        (AI|AIMoveTo self "0, 0, 0" (Game|GetPlayerCharacter 0) 5.0 false)
        (else
          (Components|Movement|StopMovementImmediately (Variables|Character|GetCharacterMovement)))))))

(fn ConstructionScript)

(fn AnimStateMachine
  (params (currentIsMoving :type Boolean) (currentIsDead :type Boolean))
  (if currentIsDead
    (Variables|Default|SetAnim%20State "NewEnumerator2")
    (elif currentIsMoving
      (Variables|Default|SetAnim%20State "NewEnumerator1")
      (else
        (Variables|Default|SetAnim%20State "NewEnumerator0"))))
  (return (Utilities|Select :Index (Variables|Default|GetAnim%20State) :NewEnumerator0 (Variables|Default|GetidleAnim) :NewEnumerator1 (Variables|Default|GetwalkLeftAnim) :NewEnumerator2 (Variables|Default|GetdeathAnim))))