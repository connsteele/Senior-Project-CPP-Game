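; Ranged enemy for a turn-based game that spends action points to damage the player.
; Overlaps on an attack sphere track whether the player's capsule is in range.
; On its turn, Tick line-traces pawns toward the player and, on a capsule hit, stops movement and applies one damage per shot by directly reducing health.
; Shots repeat each frame until points run short, then the remainder is zeroed.
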(event OnComponentBeginOverlap(rangedAttackSphere)
  (params (OverlappedComponent :type Primitive%20Component%20Object%20Reference) (OtherActor :type Actor%20Object%20Reference) (OtherComp :type Primitive%20Component%20Object%20Reference) (OtherBodyIndex :type Integer) (bFromSweep :type Boolean) (SweepResult :type Hit%20Result%20Structure%20%28by%20ref%29))
  ;[1 1 1] Set playerInRange if playuer is in range of enemy's attack sphere
  (Utilities|Casting|CastToProtagClass OtherActor)
  (Utilities|Casting|CastToCapsuleComponent OtherComp)
  (Variables|Default|SetplayerInRange true))

(event OnComponentEndOverlap(rangedAttackSphere)
  (params (OverlappedComponent :type Primitive%20Component%20Object%20Reference) (OtherActor :type Actor%20Object%20Reference) (OtherComp :type Primitive%20Component%20Object%20Reference) (OtherBodyIndex :type Integer))
  ;[1 1 1] Set playerInRange if playuer is in range of enemy's attack sphere
  (Utilities|Casting|CastToProtagClass OtherActor)
  (Utilities|Casting|CastToCapsuleComponent OtherComp)
  (Variables|Default|SetplayerInRange false))

(event EventBeginPlay
  (|CallParentFunction) ; This node is disabled and will not be called.\nDrag off pins to build functionality.
)

(event Collision|EventActorBeginOverlap
  (params (OtherActor :type Actor%20Object%20Reference))
  (|CallParentFunction OtherActor) ; This node is disabled and will not be called.\nDrag off pins to build functionality.
)

(event EventTick
  (params (DeltaSeconds :type Float%20%28single-precision%29))
  ;[1 1 1] Tick. Checks if player is in range and visible, and fires if both are true
  (|CallParentFunction DeltaSeconds)
  (if (and (Variables|Default|GetisTurn) (Variables|Default|GetplayerInRange))
    (bind _outhit (Collision|LineTraceForObjects (Transformation|GetWorldLocation (Variables|Default|GetCapsuleComponent)) (Transformation|GetWorldLocation (Variables|/Script/Engine.Character|GetCapsuleComponent (Game|GetPlayerCharacter 0))) (Utilities|Array|MakeArray "ObjectTypeQuery3") false 0 "None"))
    (bind _asprotag_class (Utilities|Casting|CastToProtagClass (.HitActor (Collision|BreakHitResult _outhit))))
    (Utilities|Casting|CastToCapsuleComponent (.HitComponent (Collision|BreakHitResult _outhit)))
    (Components|Movement|StopMovementImmediately (Variables|Character|GetCharacterMovement))
    (if (>= (Variables|Default|GetturnAP) 3e+01)
      (Variables|Default|SetturnAP (- (Variables|Default|GetturnAP) 3e+01))
      (Variables|/Script/HSPGame.Base2DCharacter|SetcurrHealth _asprotag_class (- (Variables|/Script/HSPGame.Base2DCharacter|GetcurrHealth _asprotag_class) 1.0)) ; Need to end turn
      (else
        (Variables|Default|SetturnAP 0.0)))))

(fn ConstructionScript
  (|CallParentFunction))