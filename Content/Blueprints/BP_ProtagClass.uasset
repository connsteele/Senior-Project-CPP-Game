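; Protagonist Blueprint that adds the player HUD and hides static mesh actors blocking the camera's view of the character.
; A looping timer runs a capsule trace from camera to actor against WorldStatic objects, with persistent debug drawing.
; Hits are hidden directly and added to HiddenMeshes; helpers call ToggleHideMesh(false) on BP_FadeComponents.
; HitMeshes is cleared but never filled, and SetHiddenMeshes copies it over HiddenMeshes.
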(event EventBeginPlay
  (bind _returnvalue (UserInterface|CreateWidget "/Game/UI/playerHud.playerHud_C"))
  (UserInterface|Viewport|AddtoViewport _returnvalue 0)
  (Utilities|Time|SetTimerbyFunctionName 0 "UpdateFadeActors" 0.2 true) ; Call the listed function every interval set in time
)

(event Collision|EventActorBeginOverlap
  (params (OtherActor :type Actor%20Object%20Reference)))

(event EventTick
  (params (DeltaSeconds :type Float%20%28single-precision%29)))

(fn ConstructionScript)

(fn UpdateFadeActors
  (bind _capsulecomponent (Variables|Default|GetCapsuleComponent))
  (Utilities|Array|Clear (Variables|Default|GetHitMeshes))
  (bind (_outhits _returnvalue) (Class|KismetSystemLibrary|CapsuleTraceMultiforObjects (Transformation|GetWorldLocation (Variables|Default|GetCamera)) (Transformation|GetActorLocation) (Variables|/Script/Engine.CapsuleComponent|GetCapsuleRadius _capsulecomponent) (Variables|/Script/Engine.CapsuleComponent|GetCapsuleHalfHeight _capsulecomponent) (Utilities|Array|MakeArray "ObjectTypeQuery1") false 0 "Persistent" true))
  (if _returnvalue
    (for _array_element _outhits
      (bind _asstatic_mesh_actor (Utilities|Casting|CastToStaticMeshActor (.HitActor (Collision|BreakHitResult _array_element))))
      (Development|PrintString "Hit Static Mesh")
      (Rendering|SetActorHiddenInGame _asstatic_mesh_actor true)
      (Utilities|Array|AddUnique (Variables|Default|GetHiddenMeshes) _asstatic_mesh_actor)
      (CallFunction|SetShownMeshes)
      (CallFunction|SetHiddenMeshes))
    (else
      (CallFunction|SetShownMeshes))))

(fn SetShownMeshes
  (for _array_element (Variables|Default|GetHiddenMeshes)
    (if (not (Utilities|Array|ContainsItem (Variables|Default|GetHitMeshes) _array_element))
      (for _array_element_2 (Actor|GetComponentsByClass _array_element "/Game/Blueprints/BP_FadeComponent.BP_FadeComponent_C")
        (Default|ToggleHideMesh _array_element_2 false)))))

(fn SetHiddenMeshes
  (bind _output_get (Variables|Default|SetHiddenMeshes (Variables|Default|GetHitMeshes)))
  (for _array_element _output_get
    (for _array_element_2 (Actor|GetComponentsByClass _array_element "/Game/Blueprints/BP_FadeComponent.BP_FadeComponent_C")
      (Default|ToggleHideMesh _array_element_2 false))))